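; Paper2D player character for side-view 2D play, with jumping and horizontal movement.
; The Horizontal axis feeds movement input along world X, and the Jump action starts and stops the jump.
; A Control Rotation macro branches on the axis sign, flipping controller yaw between 0 and 180 degrees to face the travel direction.
; Its outputs switch the sprite between Idle and Run flipbooks, with no separate jump animation.
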(event EventBeginPlay)

(event Collision|EventActorBeginOverlap
  (params (OtherActor :type Actor%20Object%20Reference)))

(event EventTick
  (params (DeltaSeconds :type Float%20%28single-precision%29)))

(event Input|ActionEvents|InputActionJump
  (params (Key :type Key%20Structure :default "None"))
  ;[1 1 1] Salto
  (:Pressed
    (Character|Jump))
  (:Released
    (Character|StopJumping)))

(event Input|AxisEvents|InputAxisHorizontal
  (params (AxisValue :type Float%20%28single-precision%29))
  ;[1 1 1] Movimiento
  (Pawn|Input|AddMovementInput "1.000000, 0, 0" AxisValue false)
  (|ControlRotation AxisValue
    (:Stop
      ;[1 1 1] Control de animación
      (Sprite|SetFlipbook (Variables|Default|GetSprite) "/Game/Sprites/Character/Idle/Idle.Idle"))
    (:Rigth
      (Sprite|SetFlipbook (Variables|Default|GetSprite) "/Game/Sprites/Character/Run/Run.Run" :!label _label))
    (:Left
      (goto _label))))

(fn ConstructionScript)